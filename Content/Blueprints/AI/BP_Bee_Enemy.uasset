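; BP_Bee_Enemy is a bee enemy that moves back and forth, hurts the player on contact and dies when jumped on.
; Capsule hits apply damage to the player; hits on the head box destroy the bee and launch player 0's character upward.
; The construction script feeds two relative locations and a travel duration into an InterpToMovement component to define the patrol.
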(event `self.CapsuleComponent.OnComponentHit`
  (params (HitComponent :type "PrimitiveComponent Object Reference") (OtherActor :type "Actor Object Reference") (OtherComp :type "PrimitiveComponent Object Reference") (NormalImpulse :type "Vector Structure") (Hit :type "HitResult Structure (by ref)"))
  ;[1 1 1] Damage Player
  (`/Game/Blueprints/MacroLib/MacroLibrary.IsPlayer` OtherActor
    (:`IsPlayer`
      (`GameplayStatics.ApplyDamage` OtherActor (`self.DamageValue`)))))

(event `self.BoxCollisionOnHead.OnComponentHit`
  (params (HitComponent :type "PrimitiveComponent Object Reference") (OtherActor :type "Actor Object Reference") (OtherComp :type "PrimitiveComponent Object Reference") (NormalImpulse :type "Vector Structure") (Hit :type "HitResult Structure (by ref)"))
  (bind _returnvalue (`GameplayStatics.GetPlayerPawn` 0))
  ;[1 1 1] Player Jump on Enemy
  (`/Game/Blueprints/MacroLib/MacroLibrary.IsPlayer` OtherActor
    (:`IsPlayer`
      (`self.K2_DestroyActor`)
      (if (== OtherActor _returnvalue)
        (bind _ascharacter (cast `Character` _returnvalue))
        (`self.LaunchCharacter` _ascharacter (`KismetMathLibrary.MakeVector` 0.0 0.0 (`self.LaunchVelocity`)) false false)))))

(fn `UserConstructionScript`
  (bind _interptomovement (`self.InterpToMovement`))
  ;[1 1 1] Back And Forth Movement
  (set `InterpToMovementComponent.ControlPoints` (`|MakeArray` (make `InterpControlPoint` (`self.Location_1`)) (make `InterpControlPoint` (`self.Location_2`))) _interptomovement)
  (set `InterpToMovementComponent.Duration` (`self.DelayToMove`) _interptomovement))