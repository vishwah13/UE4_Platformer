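; Crab enemy that patrols between two target actors, damages the player on contact and dies when jumped on.
; BeginPlay starts an endless AIMoveTo loop between the targets, pausing after each move and carrying on even if it fails.
; Capsule hits on the player apply damage, while Box hits destroy the crab and launch the player upward if it is player 0's pawn.
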(event `self.ReceiveBeginPlay`
  (`|AIMoveTo` self (0.0 0.0 0.0) (`self.targetTransform_1`) :!label _label
    (:`OnSuccess`
      _)
    (:`OnFail`
      _))
  (`KismetSystemLibrary.Delay` (`self.DelayToMove`))
  (`|AIMoveTo` self (0.0 0.0 0.0) (`self.targetTransform_2`)
    (:`OnSuccess`
      _)
    (:`OnFail`
      _))
  (`KismetSystemLibrary.Delay` (`self.DelayToMove`))
  (goto _label))

(event `self.CapsuleComponent.OnComponentHit`
  (params (HitComponent :type "PrimitiveComponent Object Reference") (OtherActor :type "Actor Object Reference") (OtherComp :type "PrimitiveComponent Object Reference") (NormalImpulse :type "Vector Structure") (Hit :type "HitResult Structure (by ref)"))
  ;[1 1 1] Damage Player and Destroy self
  (`/Game/Blueprints/MacroLib/MacroLibrary.IsPlayer` OtherActor
    (:`IsPlayer`
      (`GameplayStatics.ApplyDamage` OtherActor (`self.DamageValue`)))))

(event `self.Box.OnComponentHit`
  (params (HitComponent :type "PrimitiveComponent Object Reference") (OtherActor :type "Actor Object Reference") (OtherComp :type "PrimitiveComponent Object Reference") (NormalImpulse :type "Vector Structure") (Hit :type "HitResult Structure (by ref)"))
  (bind _returnvalue (`GameplayStatics.GetPlayerPawn` 0))
  ;[1 1 1] Player Jump On Enemy
  (`/Game/Blueprints/MacroLib/MacroLibrary.IsPlayer` OtherActor
    (:`IsPlayer`
      (`self.K2_DestroyActor`)
      (if (== OtherActor _returnvalue)
        (bind _ascharacter (cast `Character` _returnvalue))
        (`self.LaunchCharacter` _ascharacter (`KismetMathLibrary.MakeVector` 0.0 0.0 (`self.LaunchVelocity`)) false false)))))

(fn `UserConstructionScript`)