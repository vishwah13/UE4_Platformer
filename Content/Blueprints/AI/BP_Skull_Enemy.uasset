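; Skull enemy that chases the player, bites on contact and can be killed with a jump.
; A short-delay AI Move To loop re-targets the player character whether the move succeeds or fails.
; Capsule hits on the player play a bite montage and apply damage.
; Box hits from the player, intended as jumps on the enemy, destroy it and launch the player upward as a bounce.
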(event `self.ReceiveBeginPlay`
  ;[1 1 1] AI Navigation
  (`|AIMoveTo` self (0.0 0.0 0.0) (`GameplayStatics.GetPlayerCharacter` 0) :!label _label
    (:`OnSuccess`
      _)
    (:`OnFail`
      _))
  (`KismetSystemLibrary.Delay` 0.2)
  (goto _label))

(event `self.CapsuleComponent.OnComponentHit`
  (params (HitComponent :type "PrimitiveComponent Object Reference") (OtherActor :type "Actor Object Reference") (OtherComp :type "PrimitiveComponent Object Reference") (NormalImpulse :type "Vector Structure") (Hit :type "HitResult Structure (by ref)"))
  ;[1 1 1] Damage Player
  (`/Game/Blueprints/MacroLib/MacroLibrary.IsPlayer` OtherActor
    (:`IsPlayer`
      (`|PlayMontage` (`self.Mesh`) "/Game/Animations/Enemies/Skull_Bite_MOntage.Skull_Bite_MOntage"
        (:`then`
          (`GameplayStatics.ApplyDamage` OtherActor (`self.DamageValue`)))))))

(event `self.Box.OnComponentHit`
  (params (HitComponent :type "PrimitiveComponent Object Reference") (OtherActor :type "Actor Object Reference") (OtherComp :type "PrimitiveComponent Object Reference") (NormalImpulse :type "Vector Structure") (Hit :type "HitResult Structure (by ref)"))
  (bind _returnvalue (`GameplayStatics.GetPlayerPawn` 0))
  ;[1 1 1] Player Jump on Enemy
  (`/Game/Blueprints/MacroLib/MacroLibrary.IsPlayer` OtherActor
    (:`IsPlayer`
      (`self.K2_DestroyActor`)
      (if (== OtherActor _returnvalue)
        (bind _ascharacter (cast `Character` _returnvalue))
        (`self.LaunchCharacter` _ascharacter (`KismetMathLibrary.MakeVector` 0.0 0.0 (`self.LaunchVelocity`)) false false)))))

(fn `UserConstructionScript`)