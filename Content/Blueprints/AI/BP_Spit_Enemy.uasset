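; Spitting enemy character that fires projectiles while turning to face the player, and dies when jumped on.
; From BeginPlay it loops the spit montage, spawning BP_Enemy_Spit at ProjectileSpawnPoint on completion, then waiting ProjectileTime.
; Tick plays the Interpolation timeline, which lerps only the capsule's yaw toward the player pawn.
; A player hit on the head box destroys the enemy and launches the player upward.
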(event `self.ReceiveBeginPlay`
  ;[1 1 1] Shoot Projectile towards player
  (`|PlayMontage` (`self.Mesh`) "/Game/Animations/Enemies/Spit_Montage.Spit_Montage" :!label _label
    (:`OnCompleted`
      (`self.SpawnProjectile`)
      (`KismetSystemLibrary.Delay` (`self.Projectile_Time`))
      (goto _label))))

(event `Rotae Towards`
  (bind _returnvalue (`GameplayStatics.GetPlayerPawn` 0))
  (bind _capsulecomponent (`self.CapsuleComponent`))
  (bind (_returnvalue_roll _returnvalue_pitch _returnvalue_yaw) (`KismetMathLibrary.BreakRotator` (`SceneComponent.K2_GetComponentRotation` _capsulecomponent)))
  (bind (_returnvalue_roll_2 _returnvalue_pitch_2 _returnvalue_yaw_2) (`KismetMathLibrary.BreakRotator` (`KismetMathLibrary.FindLookAtRotation` (`SceneComponent.K2_GetComponentLocation` _capsulecomponent) (`self.K2_GetActorLocation` _returnvalue))))
  ;[1 1 1] Turn Towards Player
  (bind (_direction _turnaplha) (`Timeline|Interpolation`)
    (:`Update`
      (`/Engine/EditorBlueprintResources/StandardMacros.IsValid` _returnvalue
        (:`Is Valid`
          (`SceneComponent.K2_SetWorldRotation` (`self.CapsuleComponent`) (`KismetMathLibrary.MakeRotator` _returnvalue_roll _returnvalue_pitch (`KismetMathLibrary.Lerp` _returnvalue_yaw _returnvalue_yaw_2 _turnaplha)) false false))))))

(event `self.ReceiveTick`
  (params (DeltaSeconds :type "Float (single-precision)"))
  ;[1 1 1] Turn Towards Player
  (`self.Rotae Towards`))

(event `self.BoxCollisionOnHead.OnComponentHit`
  (params (HitComponent :type "PrimitiveComponent Object Reference") (OtherActor :type "Actor Object Reference") (OtherComp :type "PrimitiveComponent Object Reference") (NormalImpulse :type "Vector Structure") (Hit :type "HitResult Structure (by ref)"))
  (bind _returnvalue (`GameplayStatics.GetPlayerPawn` 0))
  ;[1 1 1] Player jump on enemy
  (`/Game/Blueprints/MacroLib/MacroLibrary.IsPlayer` OtherActor
    (:`IsPlayer`
      (`self.K2_DestroyActor`)
      (if (== OtherActor _returnvalue)
        (bind _ascharacter (cast `Character` _returnvalue))
        (`self.LaunchCharacter` _ascharacter (`KismetMathLibrary.MakeVector` 0.0 0.0 (`self.LaunchVelocity`)) false false)))))

(fn `SpawnProjectile`
  (bind _projectile_spawnpoint (`self.Projectile SpawnPoint`))
  (`|SpawnActorFromClass` "/Game/Blueprints/Actors/Obstacles/BP_Enemy_Spit.BP_Enemy_Spit_C" (`KismetMathLibrary.MakeTransform` (`SceneComponent.K2_GetComponentLocation` _projectile_spawnpoint) (`SceneComponent.K2_GetComponentRotation` _projectile_spawnpoint) (`KismetMathLibrary.Conv_DoubleToVector` (`self.ProjectileScale`))) "Undefined" "OverrideRootScale" null null))

(fn `UserConstructionScript`)