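; BP_NPC is a non-player character that offers dialog when BP_Player enters its interaction box.
; Overlap shows a text render and creates a W_DialogUI widget; leaving hides the text and removes the widget.
; EventDialogOccurs passes NPCText to the widget, reveals it and advances TextRow, removing the widget when the next row would exceed the last.
; A DoOnce gates each step and is reset immediately afterwards.
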(event `self.BoxCollisionToInteract.OnComponentBeginOverlap`
  (params (OverlappedComponent :type "PrimitiveComponent Object Reference") (OtherActor :type "Actor Object Reference") (OtherComp :type "PrimitiveComponent Object Reference") (OtherBodyIndex :type Integer) (bFromSweep :type Boolean) (SweepResult :type "HitResult Structure (by ref)"))
  (cast `/Game/Blueprints/Characters/BP_Player` OtherActor)
  (`SceneComponent.SetHiddenInGame` (`self.TextRender`) false false)
  (bind _returnvalue (`|CreateWidget` "/Game/Blueprints/UI/W_DialogUI.W_DialogUI_C"))
  (bind _output_get (set `self.DialogUI` _returnvalue))
  (`UserWidget.AddToViewport` _output_get 0))

(event `self.BoxCollisionToInteract.OnComponentEndOverlap`
  (params (OverlappedComponent :type "PrimitiveComponent Object Reference") (OtherActor :type "Actor Object Reference") (OtherComp :type "PrimitiveComponent Object Reference") (OtherBodyIndex :type Integer))
  (bind _dialogui (`self.DialogUI`))
  (cast `/Game/Blueprints/Characters/BP_Player` OtherActor)
  (`SceneComponent.SetHiddenInGame` (`self.TextRender`) true false)
  (`/Engine/EditorBlueprintResources/StandardMacros.IsValid` _dialogui
    (:`Is Valid`
      (`Widget.RemoveFromParent` _dialogui))))

(event `/Game/Blueprints/Interfaces/NPC_Interact.EventDialogOccurs`
  (bind _returnvalue (+ (`/Game/Blueprints/UI/W_DialogUI.TextRow` (`self.DialogUI`)) 1))
  (`/Engine/EditorBlueprintResources/StandardMacros.DoOnce` false :!label _label
    (:`Completed`
      (set `/Game/Blueprints/UI/W_DialogUI.Text` (`self.NPCText`) (`self.DialogUI`))
      (`Widget.SetVisibility` (`/Game/Blueprints/UI/W_DialogUI.TextBlock_0` (`self.DialogUI`)) "Visible")
      (`Widget.SetVisibility` (`/Game/Blueprints/UI/W_DialogUI.Image_0` (`self.DialogUI`)) "Visible")
      (if (> _returnvalue (- (`KismetArrayLibrary.Array_Length` (`self.NPCText`)) 1))
        (`Widget.RemoveFromParent` (`self.DialogUI`))
        (`self.ResetDialog`)
        (else
          (set `/Game/Blueprints/UI/W_DialogUI.TextRow` _returnvalue (`self.DialogUI`))
          (`self.ResetDialog`))))))

(event `ResetDialog`
  (goto _label :!via `Reset`))

(fn `UserConstructionScript`)