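; BP_NormalNPC is an NPC Blueprint with health tracking and a landing trace.
; DecreaseHealth subtracts damage, while IsAlive returns true when Health is zero or below, the inverse of its name.
; LandingTrace casts a debug-drawn Visibility line from the capsule along the control rotation's up vector, scaled by TraceRange.
; On a blocking hit it moves TargetPoint to the impact normal vector rather than the impact point.
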(fn `DecreaseHealth`
  (params (DamageAmount :type "Float (double-precision)"))
  (set `self.Health` (- (`self.Health`) DamageAmount)))

(fn `IsAlive`
  (returns (Result :type Boolean))
  (return (<= (`self.Health`) 0.0)))

(fn `Landing Trace`
  (bind _returnvalue (`SceneComponent.K2_GetComponentLocation` (`self.CapsuleComponent`)))
  (bind _outhit (`KismetSystemLibrary.LineTraceSingle` :`Start` _returnvalue :`End` (+ _returnvalue (* (`KismetMathLibrary.GetUpVector` (`self.GetControlRotation`)) (`self.TraceRange`))) :`TraceChannel` "TraceTypeQuery1" :`DrawDebugType` "ForDuration"))
  (bind (_bblockinghit _binitialoverlap _time _distance _location _impactpoint _normal _impactnormal) (`GameplayStatics.BreakHitResult` _outhit))
  (if _bblockinghit
    (`self.K2_SetActorLocation` (`self.TargetPoint`) _impactnormal false false)))

(fn `UserConstructionScript`)