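; BP_RotatingPlatform is a platform actor whose mesh rotates in pitch, driven by the PlatformRotate timeline started on BeginPlay.
; Each timeline update sets relative pitch by lerping from zero toward current pitch plus RotationRate, clearing roll and yaw.
; The same update path feeds a RotateTime delay that restarts the timeline.
; An unconnected node that would set RotatingMovement's rotation rate never runs.
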(event `self.ReceiveBeginPlay`
  (bind (_relativerotation_roll _relativerotation_pitch) (`KismetMathLibrary.BreakRotator` (`SceneComponent.RelativeRotation` (`self.PlatformMesh`))))
  (bind (_direction _rotate_alpha) (`Timeline|PlatformRotate` :!label _label)
    (:`Update`
      (`SceneComponent.K2_SetRelativeRotation` (`self.PlatformMesh`) (`KismetMathLibrary.MakeRotator` 0.0 (`KismetMathLibrary.Lerp` 0.0 (+ _relativerotation_pitch (`self.RotationRate`)) _rotate_alpha)) false false)
      (`KismetSystemLibrary.Delay` (`self.RotateTime`))
      (goto _label :!via `PlayFromStart`))))

(fn `UserConstructionScript`)