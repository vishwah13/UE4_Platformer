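; BP_VictoryZone is a trigger volume that completes the level when the player overlaps its box.
; It looks up the current level name in an ordered LevelNames array and opens the next entry by name.
; When the current level is the last entry, it opens the level named FinalLevel instead.
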(event `self.Box.OnComponentBeginOverlap`
  (params (OverlappedComponent :type "PrimitiveComponent Object Reference") (OtherActor :type "Actor Object Reference") (OtherComp :type "PrimitiveComponent Object Reference") (OtherBodyIndex :type Integer) (bFromSweep :type Boolean) (SweepResult :type "HitResult Structure (by ref)"))
  (`/Game/Blueprints/MacroLib/MacroLibrary.IsPlayer` OtherActor
    (:`IsPlayer`
      (`self.CompleteLevel`))))

(fn `CompleteLevel`
  (if (`self.IsFinalLevel`)
    (`GameplayStatics.OpenLevel` "FinalLevel")
    (else
      (`self.LoadNextLevel`))))

(fn `GetCurrentLevelIndex`
  (returns (`Return Value` :type Integer))
  (bind _returnvalue (`GameplayStatics.GetCurrentLevelName` true))
  (return (`KismetArrayLibrary.Array_Find` (`self.LevelNames`) (`KismetStringLibrary.Conv_StringToName` _returnvalue))))

(fn `GetNextLevelName`
  (returns (Output :type Name))
  (return (`|GetArrayItem` (`self.LevelNames`) (+ (`self.GetCurrentLevelIndex`) 1))))

(fn `IsFinalLevel`
  (returns (`Return boolien` :type Boolean))
  (return (== (`KismetArrayLibrary.Array_LastIndex` (`self.LevelNames`)) (`self.GetCurrentLevelIndex`))))

(fn `LoadNextLevel`
  (`GameplayStatics.OpenLevel` (`self.GetNextLevelName`)))

(fn `UserConstructionScript`)