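; BP_SawBlade is a moving obstacle actor that damages actors on contact.
; Its construction script builds an InterpToMovement path from two relative control points, Location1 and Location2, and sets the movement Duration from a variable.
; The Hit event applies DamageValue to whatever actor it collides with.
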(event `self.ReceiveHit`
  (params (MyComp :type "PrimitiveComponent Object Reference") (Other :type "Actor Object Reference") (OtherComp :type "PrimitiveComponent Object Reference") (bSelfMoved :type Boolean) (HitLocation :type "Vector Structure") (HitNormal :type "Vector Structure") (NormalImpulse :type "Vector Structure") (Hit :type "HitResult Structure (by ref)"))
  (`GameplayStatics.ApplyDamage` Other (`self.DamageValue`)))

(fn `UserConstructionScript`
  (bind _interptomovement (`self.InterpToMovement`))
  (set `InterpToMovementComponent.ControlPoints` (`|MakeArray` (make `InterpControlPoint` (`self.Location_1`) true) (make `InterpControlPoint` (`self.Location_2`) true)) _interptomovement)
  (set `InterpToMovementComponent.Duration` (`self.Duration`) _interptomovement))