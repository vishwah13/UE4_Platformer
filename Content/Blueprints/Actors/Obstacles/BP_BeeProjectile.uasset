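; BP_BeeProjectile is a bee projectile obstacle that damages what it hits and can be jumped on by the player.
; It destroys itself after a set lifetime, or on a hit after applying its configured damage.
; A separate Box component handles player contact as a stomp, destroying the projectile and launching the player 0 character with a set vertical velocity.
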(event `self.ReceiveBeginPlay`
  (`KismetSystemLibrary.Delay` (`self.DestroyTime`))
  (`self.K2_DestroyActor`))

(event `self.ReceiveHit`
  (params (MyComp :type "PrimitiveComponent Object Reference") (Other :type "Actor Object Reference") (OtherComp :type "PrimitiveComponent Object Reference") (bSelfMoved :type Boolean) (HitLocation :type "Vector Structure") (HitNormal :type "Vector Structure") (NormalImpulse :type "Vector Structure") (Hit :type "HitResult Structure (by ref)"))
  (`GameplayStatics.ApplyDamage` Other (`self.DamageValue`) null null "/Script/Engine.DamageType")
  (`self.K2_DestroyActor`))

(event `self.Box.OnComponentHit`
  (params (HitComponent :type "PrimitiveComponent Object Reference") (OtherActor :type "Actor Object Reference") (OtherComp :type "PrimitiveComponent Object Reference") (NormalImpulse :type "Vector Structure") (Hit :type "HitResult Structure (by ref)"))
  (bind _returnvalue (`GameplayStatics.GetPlayerPawn` 0))
  ;[1 1 1] Player Jump on Enemy
  (`/Game/Blueprints/MacroLib/MacroLibrary.IsPlayer` OtherActor
    (:`IsPlayer`
      (`self.K2_DestroyActor`)
      (if (== OtherActor _returnvalue)
        (bind _ascharacter (cast `Character` _returnvalue))
        (`Character.LaunchCharacter` _ascharacter (`KismetMathLibrary.MakeVector` 0.0 0.0 (`self.LaunchVelocity`)) false false)))))

(fn `UserConstructionScript`)