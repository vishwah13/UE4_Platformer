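; BP_LaunchPad is a launch pad obstacle that throws the player character upward.
; Any overlap with its Box plays a bounce montage on BouncerMesh, then launches the overlapping actor vertically by LaunchVelocity if it is player 0's Character.
; A LaunchPlayer function repeats the launch logic but is not called here, and it reads LunchVelocity instead of its LaunchVelocity input.
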(event `self.Box.OnComponentBeginOverlap`
  (params (OverlappedComponent :type "PrimitiveComponent Object Reference") (OtherActor :type "Actor Object Reference") (OtherComp :type "PrimitiveComponent Object Reference") (OtherBodyIndex :type Integer) (bFromSweep :type Boolean) (SweepResult :type "HitResult Structure (by ref)"))
  (bind _returnvalue (`GameplayStatics.GetPlayerPawn` 0))
  (`|PlayMontage` (`self.BouncerMesh`) "/Game/Animations/Bounce_Maontage.Bounce_Maontage"
    (:`then`
      (if (== OtherActor _returnvalue)
        (bind _ascharacter (cast `Character` _returnvalue))
        (`Character.LaunchCharacter` _ascharacter (`KismetMathLibrary.MakeVector` 0.0 0.0 (`self.LaunchVelocity`)) false false)))))

(fn `LaunchPlayer`
  (params (A :type "Object Object Reference") (LunchVelocity :type "Float (double-precision)"))
  (bind _returnvalue (`GameplayStatics.GetPlayerPawn` 0))
  (if (== A _returnvalue)
    (bind _ascharacter (cast `Character` _returnvalue))
    (`Character.LaunchCharacter` _ascharacter (`KismetMathLibrary.MakeVector` 0.0 0.0 LunchVelocity) false false)))

(fn `UserConstructionScript`)