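; Spike trap obstacle that plays a spike montage after the player steps into its trigger box.
; Overlap begin sets CanDamagePlayer and, after a delay, plays the montage unless one is already playing; overlap end clears the flag.
; DamagePlayer applies per-hit damage to player character 0, but nothing in this file calls it or reads the flag.
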(event `self.BoxTrigger.OnComponentBeginOverlap`
  (params (OverlappedComponent :type "PrimitiveComponent Object Reference") (OtherActor :type "Actor Object Reference") (OtherComp :type "PrimitiveComponent Object Reference") (OtherBodyIndex :type Integer) (bFromSweep :type Boolean) (SweepResult :type "HitResult Structure (by ref)"))
  (`/Game/Blueprints/MacroLib/MacroLibrary.IsPlayer` OtherActor
    (:`IsPlayer`
      (set `self.CanDamagePlayer` true)
      (`KismetSystemLibrary.Delay` (`self.SpikeTriggerTime`))
      (if (not (`self.IsAnimPlaying`))
        (`|PlayMontage` (`self.SpikeTrapMesh`) "/Game/Animations/SpikeTrap_Montage_.SpikeTrap_Montage_")))))

(event `self.BoxTrigger.OnComponentEndOverlap`
  (params (OverlappedComponent :type "PrimitiveComponent Object Reference") (OtherActor :type "Actor Object Reference") (OtherComp :type "PrimitiveComponent Object Reference") (OtherBodyIndex :type Integer))
  (`/Game/Blueprints/MacroLib/MacroLibrary.IsPlayer` OtherActor
    (:`IsPlayer`
      (set `self.CanDamagePlayer` false))))

(fn `DamagePlayer`
  (`GameplayStatics.ApplyDamage` (`GameplayStatics.GetPlayerCharacter` 0) (`self.DamagePerhit`)))

(fn `IsAnimPlaying`
  (returns (Return :type Boolean))
  (return (`AnimInstance.Montage_IsPlaying` (`SkeletalMeshComponent.GetAnimInstance` (`self.SpikeTrapMesh`)) null)))

(fn `UserConstructionScript`)