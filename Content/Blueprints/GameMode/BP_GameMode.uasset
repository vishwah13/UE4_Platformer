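; Game mode that handles player respawning, a coin tally and an intro dialog.
; Respawn fades the camera and binds to the player's destruction, which after a delay spawns and possesses a new BP_Player, then rebinds.
; BeginPlay also creates the dialog widget and, once only, shows NPC text, advancing a row and removing it after five seconds if another row exists.
; AddCoin increments the coin count.
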(event `Respawn`
  (`PlayerCameraManager.StartCameraFade` :`self` (`GameplayStatics.GetPlayerCameraManager` 0) :`FromAlpha` 1.0 :`Duration` 2.0 :`bHoldWhenFinished` true :!label _label)
  (bind _asbp_player (cast `/Game/Blueprints/Characters/BP_Player` (`GameplayStatics.GetPlayerCharacter` 0)))
  (add `self.OnDestroyed` _asbp_player (delegate `OnDestroyed_`)))

(event `self.ReceiveBeginPlay`
  (`self.Begin`)
  (goto _label))

(event `OnDestroyed_` :!signature `self.OnDestroyed`
  (params (DestroyedActor :type "Actor Object Reference"))
  (`KismetSystemLibrary.Delay` (`self.RespawnDelay`))
  (bind _returnvalue (`|SpawnActorFromClass` "/Game/Blueprints/Characters/BP_Player.BP_Player_C" (`self.SpawnTransform`) "Undefined" "OverrideRootScale" null null))
  (`Controller.Possess` (`GameplayStatics.GetPlayerController` 0) _returnvalue)
  (`self.Respawn`))

(event `Begin`
  (bind _returnvalue (`|CreateWidget` "/Game/Blueprints/UI/W_DialogUI.W_DialogUI_C"))
  (bind _output_get (set `self.DialogUI` _returnvalue))
  (`UserWidget.AddToViewport` _output_get 0)
  (`self.EventDialogOccurs`))

(event `self.EventDialogOccurs`
  (bind _returnvalue (+ (`/Game/Blueprints/UI/W_DialogUI.TextRow` (`self.DialogUI`)) 1))
  (`/Engine/EditorBlueprintResources/StandardMacros.DoOnce` false
    (:`Completed`
      (set `/Game/Blueprints/UI/W_DialogUI.Text` (`self.NPCText`) (`self.DialogUI`))
      (`Widget.SetVisibility` (`/Game/Blueprints/UI/W_DialogUI.TextBlock_0` (`self.DialogUI`)) "Visible")
      (`Widget.SetVisibility` (`/Game/Blueprints/UI/W_DialogUI.Image_0` (`self.DialogUI`)) "Visible")
      (if (not (> _returnvalue (- (`KismetArrayLibrary.Array_Length` (`self.NPCText`)) 1)))
        (set `/Game/Blueprints/UI/W_DialogUI.TextRow` _returnvalue (`self.DialogUI`))
        (`KismetSystemLibrary.Delay` 5.0)
        (`Widget.RemoveFromParent` (`self.DialogUI`))))))

(fn `AddCoin`
  (params (Value :type Integer))
  (set `self.NumberOfCoins` (+ (`self.NumberOfCoins`) Value)))

(fn `UserConstructionScript`)